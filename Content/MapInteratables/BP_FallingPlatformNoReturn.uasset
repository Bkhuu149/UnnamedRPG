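; BP_FallingPlatformNoReturn is an interactable platform that starts falling when a MyRPGCharacter hits it and has no return logic.
; The Hit event sets a Falling flag, and Tick calls Fall while it is set.
; Fall applies a fixed, frame-rate-dependent downward swept offset, clears the flag on a blocking hit, and prints the hit actor's name.
; An unconnected Delay leading into the fall check never runs.
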(event EventBeginPlay)

(event EventTick
  (params (DeltaSeconds :type Float%20%28single-precision%29))
  (if (Variables|Default|GetFalling)
    (CallFunction|Fall)))

(event Collision|EventHit
  (params (MyComp :type Primitive%20Component%20Object%20Reference) (Other :type Actor%20Object%20Reference) (OtherComp :type Primitive%20Component%20Object%20Reference) (bSelfMoved :type Boolean) (HitLocation :type Vector :default "0, 0, 0") (HitNormal :type Vector :default "0, 0, 0") (NormalImpulse :type Vector :default "0, 0, 0") (Hit :type Hit%20Result%20Structure%20%28by%20ref%29))
  (Utilities|Casting|CastToMyRPGCharacter Other)
  (Variables|Default|SetFalling true))

(fn ConstructionScript)

(fn Fall
  (bind _sweephitresult (Transformation|AddActorWorldOffset "0.000000,0.000000,-10.000000" true))
  (Variables|Default|SetFalling (not (.bblockinghit _sweephitresult)))
  (Development|PrintString (Utilities|GetDisplayName (.hitactor _sweephitresult)))
  (return))