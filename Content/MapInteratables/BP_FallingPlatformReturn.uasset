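; Platform actor that sinks while the player character (MyRPGCharacter) overlaps it and rises back to its start once the overlap ends.
; On BeginPlay it stores its starting location and line-traces straight down on Visibility to find the lowest point it can fall to.
; Overlap events toggle a Falling flag, and Tick calls Fall or Rise, which move it by a fixed swept step per frame, independent of delta time.
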(event EventBeginPlay
  (bind _returnvalue (Transformation|GetActorLocation))
  (bind _outhit (Collision|LineTraceByChannel _returnvalue (+ _returnvalue "0.000000,0.000000,-3400000.000000") "TraceTypeQuery1" false 0 "ForDuration"))
  (Variables|Default|SetFallTo (.location _outhit))
  (Variables|Default|SetStartingPos (Transformation|GetActorLocation)))

(event Collision|EventActorBeginOverlap
  (params (OtherActor :type Actor%20Object%20Reference))
  (Utilities|Casting|CastToMyRPGCharacter OtherActor)
  (Variables|Default|SetFalling true))

(event EventTick
  (params (DeltaSeconds :type Float%20%28single-precision%29))
  (if (Variables|Default|GetFalling)
    (CallFunction|Fall)
    (else
      (CallFunction|Rise))))

(event Collision|EventActorEndOverlap
  (params (OtherActor :type Actor%20Object%20Reference))
  (Utilities|Casting|CastToMyRPGCharacter OtherActor)
  (Variables|Default|SetFalling false))

(fn ConstructionScript)

(fn Fall
  (if (> (.z (Transformation|GetActorLocation)) (.z (Variables|Default|GetFallTo)))
    (Transformation|AddActorWorldOffset "0.000000,0.000000,-2.000000" true)
    (return)))

(fn Rise
  (if (< (.z (Transformation|GetActorLocation)) (.z (Variables|Default|GetStartingPos)))
    (Transformation|AddActorWorldOffset "0.000000,0.000000,2.000000" true)
    (return)))