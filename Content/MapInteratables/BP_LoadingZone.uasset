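; BP_LoadingZone is a trigger actor that sends the player to another level when their character overlaps it.
; On overlap it shows a LoadingScreen widget, waits a few seconds, then passes its ExitTag to BP_ThirdPersonGameMode as PlayerStartTag before opening LevelToLoad by name.
; BeginPlay prints a red warning if no level is configured.
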(event EventBeginPlay
  (if (== (Variables|Default|GetLevelToLoad) "")
    (Development|PrintString "WARNING: A loading zone is not configured with a level to load, FIX THIS" true true "(R=1.000000,G=0.000000,B=0.000000,A=1.000000)")))

(event Collision|EventActorBeginOverlap
  (params (OtherActor :type Actor%20Object%20Reference))
  (Utilities|Casting|CastToMyRPGCharacter OtherActor)
  (bind _returnvalue (UserInterface|CreateWidget "/Game/Widgets/LoadingScreen.LoadingScreen_C"))
  (UserInterface|Viewport|AddtoViewport _returnvalue 0)
  (Utilities|FlowControl|Delay 3.0)
  (bind _asbp_third_person_game_mode (Utilities|Casting|CastToBP_ThirdPersonGameMode (Game|GetGameMode)))
  (Variables|/Game/ThirdPerson/Blueprints/BP_ThirdPersonGameMode.BP_ThirdPersonGameMode_C|SetPlayerStartTag _asbp_third_person_game_mode (Variables|Default|GetExitTag))
  (Game|OpenLevel(byName) (Variables|Default|GetLevelToLoad)))

(fn ConstructionScript)