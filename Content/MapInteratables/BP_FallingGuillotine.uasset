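; BP_FallingGuillotine is a map hazard that repeatedly drops and damages any RPGBaseClass actor that begins overlapping it.
; BeginPlay stores its start position and sets the drop target slightly below the first hit of a Visibility trace toward a fixed world point far below the origin.
; A Delay in Tick repeatedly restarts a Timeline, whose track lerps the actor between the two points without sweeping.
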(event EventBeginPlay
  (bind _returnvalue (Transformation|GetActorLocation))
  (Variables|Default|SetCurrentPosition _returnvalue)
  (bind _outhits (Collision|MultiLineTraceByChannel _returnvalue "0.000000,0.000000,-100000.000000" "TraceTypeQuery1" false 0 "None"))
  (Variables|Default|SetFallTo (+ (.impactpoint (Utilities|Array|Get(acopy) _outhits)) "0.000000,0.000000,-125.000000")))

(event EventTick
  (params (DeltaSeconds :type Float%20%28single-precision%29))
  (Utilities|FlowControl|Delay 2.0)
  (bind _guillotine_track (Timeline|GuillotineTimeline PlayFromStart)
    (:Update
      (Transformation|SetActorLocation (Math|Vector|Lerp(Vector) (Variables|Default|GetCurrentPosition) (Variables|Default|GetFallTo) _guillotine_track) false false))))

(event Collision|EventActorBeginOverlap
  (params (OtherActor :type Actor%20Object%20Reference))
  (bind _asrpgbase_class (Utilities|Casting|CastToRPGBaseClass OtherActor))
  (Game|Damage|ApplyDamage _asrpgbase_class (Variables|Default|GetDamage) 0 self (Variables|Default|GetMyType)))

(fn ConstructionScript)