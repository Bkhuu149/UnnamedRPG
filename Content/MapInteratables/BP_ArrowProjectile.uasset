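; BP_ArrowProjectile is an arrow actor that flies forward and damages characters it overlaps.
; Tick moves it along its forward vector by Speed each frame, without sweeping or delta-time scaling.
; On overlap with an RPGBaseClass actor other than its owner, it applies fixed damage credited to the owner, prints a debug "Hit" message and destroys itself.
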(event EventBeginPlay)

(event Collision|EventActorBeginOverlap
  (params (OtherActor :type Actor%20Object%20Reference))
  (if (!= OtherActor (Components|GetOwner))
    (bind _asrpgbase_class (Utilities|Casting|CastToRPGBaseClass OtherActor))
    (Game|Damage|ApplyDamage _asrpgbase_class 1e+01 0 (Components|GetOwner) "/Game/Weapons/DamageTypes/MyDamageType_None.MyDamageType_None_C")
    (Development|PrintString "Hit")
    (Actor|DestroyActor)))

(event EventTick
  (params (DeltaSeconds :type Float%20%28single-precision%29))
  (Transformation|SetActorLocation (+ (Transformation|GetActorLocation) (* (Transformation|GetActorForwardVector) (Variables|Default|GetSpeed))) false false))

(fn ConstructionScript)