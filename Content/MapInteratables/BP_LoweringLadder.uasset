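; BP_LoweringLadder is an interactable ladder that lowers and raises between its starting position and the surface below it.
; BeginPlay saves the top position and finds the bottom with a downward line trace, drawn for debugging.
; TryLower stops a moving ladder or restarts a stopped one opposite to its last direction, lowering first.
; Tick moves it by a fixed swept step per frame, so speed is frame-rate dependent, and stops it at either limit.
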(event Custom|TryLower
  (switch Utilities|FlowControl|Switch|SwitchonEnumLadderState (Variables|Default|GetLadderEnum)
    (:NewEnumerator0
      (Variables|Default|SetLastMovement "NewEnumerator0")
      (Variables|Default|SetLadderEnum "NewEnumerator2" :!label _label))
    (:NewEnumerator1
      (Variables|Default|SetLastMovement "NewEnumerator1")
      (goto _label))
    (:NewEnumerator2
      (switch Utilities|FlowControl|Switch|SwitchonEnumLadderState (Variables|Default|GetLastMovement)
        (:NewEnumerator0
          (Variables|Default|SetLadderEnum "NewEnumerator1"))
        (:NewEnumerator1
          (Variables|Default|SetLadderEnum "NewEnumerator0" :!label _label_2))
        (:NewEnumerator2
          (goto _label_2))))))

(event EventTick
  (params (DeltaSeconds :type Float%20%28single-precision%29))
  (switch Utilities|FlowControl|Switch|SwitchonEnumLadderState (Variables|Default|GetLadderEnum)
    (:NewEnumerator0
      (bind _output_get (Variables|Default|SetMoveSpeed -2.0))
      (Transformation|AddActorWorldOffset (Math|Vector|MakeVector 0.0 0.0 _output_get) true)
      (if (not (> (.z (Transformation|GetActorLocation)) (.z (Variables|Default|GetFallTo))))
        (Variables|Default|SetLastMovement (Variables|Default|GetLadderEnum) :!label _label)
        (Variables|Default|SetLadderEnum "NewEnumerator2")))
    (:NewEnumerator1
      (bind _output_get_2 (Variables|Default|SetMoveSpeed 2.0))
      (Transformation|AddActorWorldOffset (Math|Vector|MakeVector 0.0 0.0 _output_get_2) true)
      (if (not (< (.z (Transformation|GetActorLocation)) (.z (Variables|Default|GetTopPosition))))
        (goto _label)))))

(event EventBeginPlay
  (bind _returnvalue (Transformation|GetActorLocation))
  (bind _outhit (Collision|LineTraceByChannel _returnvalue (+ _returnvalue "0.000000,0.000000,-3400000.000000") "TraceTypeQuery1" false 0 "ForDuration"))
  (Variables|Default|SetFallTo (.location _outhit))
  (Variables|Default|SetTopPosition (Transformation|GetActorLocation)))

(fn ConstructionScript
  (|CallParentFunction))