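; BP_Pushable is a pushable interactable that shows its push points as construction-time arrows; its interact event is empty.
; The uncalled HandleInteractionOLD picks an in-range point via FindClosestPushTransformIndex, whose comparison actually favors the farthest.
; It validates that point with debug-drawn traces for standing room, walkable floor and blocking walls.
; It then teleports the character there and starts the push through their PushComponent, or prints the failure reason.
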(event EventBeginPlay)

(event Collision|EventActorBeginOverlap
  (params (OtherActor :type Actor%20Object%20Reference)))

(event EventTick
  (params (DeltaSeconds :type Float%20%28single-precision%29)))

(event EventOnInteracted
  (params (Player :type BP%20Third%20Person%20Character%20Object%20Reference)))

(fn ConstructionScript
  (for _array_element (Variables|Default|GetPushTransformsTemp)
    (AddComponent|AddArrowComponent false _array_element)))

(fn HandleInteractionOLD
  (params (Character :type Character%20Object%20Reference))
  (bind _capsulecomponent (Variables|/Script/Engine.Character|GetCapsuleComponent Character))
  (Utilities|IsValid Character
    (:Is%20Valid
      (bind _output_get (LocalVariables|SetPushComponent (Actor|GetComponentbyClass Character "/Game/MapInteratables/PushComponent.PushComponent_C")))
      (Utilities|IsValid _output_get
        (:Is%20Valid
          (bind _best_index (CallFunction|FindClosestPushTransformIndex (Math|Conversions|ToVector2D(Vector) (Transformation|GetActorLocation Character)) (Variables|/Game/MapInteratables/PushComponent.PushComponent_C|GetPushRange (LocalVariables|GetPushComponent))))
          (if (>= _best_index 0)
            (bind _output_get_2 (LocalVariables|SetCharacter%20New%20Transform (Math|Transform|MakeTransform (+ (.location (Math|Transform|ComposeTransforms (Utilities|Array|Get(acopy) (Variables|Default|GetPushTransformsTemp) _best_index) (Transformation|GetActorTransform))) (Math|Vector|MakeVector 0.0 0.0 (Components|Capsule|GetScaledCapsuleHalfHeight (Variables|/Script/Engine.Character|GetCapsuleComponent Character)))) (.rotation (Math|Transform|ComposeTransforms (Utilities|Array|Get(acopy) (Variables|Default|GetPushTransformsTemp) _best_index) (Transformation|GetActorTransform))) (.scale (Math|Transform|ComposeTransforms (Utilities|Array|Get(acopy) (Variables|Default|GetPushTransformsTemp) _best_index) (Transformation|GetActorTransform))))))
            (Rendering|Debug|DrawDebugSphere (.location _output_get_2) 2e+01 12 "(R=1.000000,G=0.000000,B=0.000000,A=1.000000)" 2.0 1.0)
            (bind _outhit (Collision|CapsuleTraceByChannel (+ (.location (LocalVariables|GetCharacter%20New%20Transform)) "0.000000,0.000000,70.000000") (- (.location (LocalVariables|GetCharacter%20New%20Transform)) "0.000000,0.000000,100.000000") (Components|Capsule|GetScaledCapsuleRadius _capsulecomponent) (Components|Capsule|GetScaledCapsuleHalfHeight _capsulecomponent) "TraceTypeQuery1" false 0 "ForDuration" true "(R=1.000000,G=0.000000,B=0.000000,A=1.000000)" "(R=0.000000,G=1.000000,B=0.000000,A=1.000000)" 2.0))
            (if (not (.binitialoverlap _outhit))
              (if (< (Class|CharacterMovementComponent|GetWalkableFloorZ (Variables|/Script/Engine.Character|GetCharacterMovement Character)) (.z (.impactnormal _outhit)))
                (bind _returnvalue (Collision|MultiLineTraceByChannel (Transformation|GetActorLocation) (.location (LocalVariables|GetCharacter%20New%20Transform)) "TraceTypeQuery1" false (Utilities|Array|MakeArray Character) "ForDuration" true "(R=1.000000,G=0.000000,B=0.000000,A=1.000000)" "(R=0.000000,G=1.000000,B=0.000000,A=1.000000)" 2.0))
                (if (not _returnvalue)
                  (Transformation|SetActorTransform Character (Math|Transform|MakeTransform (.location (LocalVariables|GetCharacter%20New%20Transform)) (.rotation (LocalVariables|GetCharacter%20New%20Transform)) "1.000000,1.000000,1.000000") false true)
                  (Default|BeginPush (LocalVariables|GetPushComponent) self)
                  (else
                    (Utilities|PushFailedInfo "Wall in between character and object")))
                (else
                  (Utilities|PushFailedInfo "Floor Not Walkable")))
              (else
                (Utilities|PushFailedInfo "No Room to Stand")))
            (else
              (Utilities|PushFailedInfo "No Push Transform Found"))))
        (:Is%20Not%20Valid
          (Utilities|PushFailedInfo "Character does not have push component"))))
    (:Is%20Not%20Valid
      (Utilities|PushFailedInfo "Character is invalid"))))

(fn FindClosestPushTransformIndex
  (params (Character%20Location :type Vector%202D%20Structure) (Push%20Range :type Float%20%28double-precision%29))
  (for (_array_element _array_index) 0
    (LocalVariables|SetCurrent%20Transform%20Index _array_index)
    (bind _output_get (LocalVariables|SetCurrent%20Distance%20Sq (Class|KismetMathLibrary|DistanceSquared2D (Math|Conversions|ToVector2D(Vector) (Math|Transform|TransformLocation (Transformation|GetActorTransform) (.location _array_element))) Character%20Location)))
    (if (< _output_get (Math|Float|Square Push%20Range))
      (if (or (< (LocalVariables|GetClosest%20Distance%20Sq) (LocalVariables|GetCurrent%20Distance%20Sq)) (< (LocalVariables|GetClosest%20Transform%20Index) 0))
        (LocalVariables|SetClosest%20Transform%20Index (LocalVariables|GetCurrent%20Transform%20Index))
        (LocalVariables|SetClosest%20Distance%20Sq (LocalVariables|GetCurrent%20Distance%20Sq)))))
  (return (LocalVariables|GetClosest%20Transform%20Index)))