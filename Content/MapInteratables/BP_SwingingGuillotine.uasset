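; BP_SwingingGuillotine is a map hazard that swings on its roll axis and damages characters it touches.
; BeginPlay stores the starting rotation and a target rolled 180 degrees from it.
; Tick feeds a Delay that periodically restarts a timeline, whose track lerps the actor between those rotations.
; Actor overlap applies damage to anything that casts to RPGBaseClass.
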(event EventBeginPlay
  (bind _returnvalue (Transformation|GetActorRotation))
  (bind (_roll _pitch _yaw) (Math|Rotator|BreakRotator _returnvalue))
  (Variables|Default|SetCurrentPosition _returnvalue)
  (Variables|Default|SetSwingTo (Math|Rotator|MakeRotator (+ _roll -1.8e+02) _pitch _yaw)))

(event EventTick
  (params (DeltaSeconds :type Float%20%28single-precision%29))
  (Utilities|FlowControl|Delay 4.0)
  (bind _guillotine_track (Timeline|GuillotineTimeline PlayFromStart)
    (:Update
      (Transformation|SetActorRotation (Math|Rotator|Lerp(Rotator) (Variables|Default|GetCurrentPosition) (Variables|Default|GetSwingTo) _guillotine_track)))))

(event Collision|EventActorBeginOverlap
  (params (OtherActor :type Actor%20Object%20Reference))
  (bind _asrpgbase_class (Utilities|Casting|CastToRPGBaseClass OtherActor))
  (Game|Damage|ApplyDamage _asrpgbase_class (Variables|Default|GetDamage) 0 self (Variables|Default|GetMyType)))

(fn ConstructionScript)