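; BP_Campfire is a map interactable that handles level saving and level resetting.
; BlueprintSave delegates to CustomGameInstance, while its own SaveLevel writes the current level name into the existing "slot1" PlayerSave, doing nothing if none exists.
; ResetLevel and LevelReset share a path that shows a loading screen, waits briefly and reopens the current level.
; An ObjectManager crate-saving call is left unconnected.
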(event Custom|Level%20Reset
  (bind _returnvalue (UserInterface|CreateWidget "/Game/Widgets/LoadingScreen.LoadingScreen_C"))
  (UserInterface|Viewport|AddtoViewport _returnvalue 0)
  (Utilities|FlowControl|Delay 1.0)
  (bind _returnvalue_2 (Game|GetCurrentLevelName true))
  (Game|OpenLevel(byName) (Utilities|String|StringToName _returnvalue_2)))

(event EventBeginPlay)

(event Collision|EventActorBeginOverlap
  (params (OtherActor :type Actor%20Object%20Reference)))

(event EventTick
  (params (DeltaSeconds :type Float%20%28single-precision%29)))

(event EventBlueprintSave
  (bind _ascustom_game_instance (Utilities|Casting|CastToCustomGameInstance (Game|GetGameInstance)))
  (Default|SaveLevel _ascustom_game_instance))

(event EventResetLevel
  (bind _returnvalue (UserInterface|CreateWidget "/Game/Widgets/LoadingScreen.LoadingScreen_C"))
  (UserInterface|Viewport|AddtoViewport _returnvalue 0)
  (Utilities|FlowControl|Delay 1.0)
  (bind _returnvalue_2 (Game|GetCurrentLevelName true))
  (Game|OpenLevel(byName) (Utilities|String|StringToName _returnvalue_2)))

(event EventSaveLevel
  (bind _returnvalue (SaveGame|DoesSaveGameExist "slot1"))
  (if _returnvalue
    (Development|PrintString "Saving Level..")
    (bind _returnvalue_2 (SaveGame|LoadGamefromSlot "slot1"))
    (bind _asplayer_save (Utilities|Casting|CastToPlayerSave _returnvalue_2))
    (bind _returnvalue_3 (Game|GetCurrentLevelName true))
    (Variables|/Game/ThirdPerson/Blueprints/PlayerSave.PlayerSave_C|SetLevel _asplayer_save (Utilities|String|StringToName _returnvalue_3))
    (SaveGame|SaveGametoSlot _asplayer_save "slot1")))

(fn ConstructionScript)