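; BP_Ladder is a map interactable actor that builds a ladder procedurally from Height and StepGap in its construction script.
; It scales the two side rails to Height and fills an instanced static mesh with rungs spaced by StepGap.
; Each loop pass also adds a full-height box component and arrows at the LadderTop and LadderBottom transforms.
; The event graph holds no active gameplay logic.
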(event EventBeginPlay)

(event Collision|EventActorBeginOverlap
  (params (OtherActor :type Actor%20Object%20Reference)))

(event EventTick
  (params (DeltaSeconds :type Float%20%28single-precision%29)))

(fn ConstructionScript
  (bind _height (Variables|Default|GetHeight))
  (bind _height_2 (Variables|Default|GetHeight))
  (bind _ladder_r (Variables|Default|GetLadder%20R))
  (bind _ladder_l (Variables|Default|GetLadder%20L))
  (bind _instancedstaticmesh (Variables|Default|GetInstancedStaticMesh))
  (bind _returnvalue (Transformation|GetRelativeTransform _ladder_l))
  (bind _returnvalue_2 (Transformation|GetRelativeTransform _ladder_r))
  (Transformation|SetRelativeTransform _ladder_l (Math|Transform|MakeTransform (Math|Vector|MakeVector (.x (.location _returnvalue)) (.y (.location _returnvalue)) (/ _height 2.0)) (.rotation _returnvalue) (Math|Vector|MakeVector (.x (.scale _returnvalue)) (.y (.scale _returnvalue)) (/ _height 1e+02))) false false)
  (Transformation|SetRelativeTransform _ladder_r (Math|Transform|MakeTransform (Math|Vector|MakeVector (.x (.location _returnvalue_2)) (.y (.location _returnvalue_2)) (/ _height_2 2.0)) (.rotation _returnvalue_2) (Math|Vector|MakeVector (.x (.scale _returnvalue_2)) (.y (.scale _returnvalue_2)) (/ _height_2 1e+02))) false false)
  (Variables|Default|SetTemp_Height 0.0)
  (Components|InstancedStaticMesh|ClearInstances _instancedstaticmesh)
  (while (< (Variables|Default|GetTemp_Height) (Variables|Default|GetHeight))
    (Components|InstancedStaticMesh|AddInstance _instancedstaticmesh (Math|Transform|MakeTransform (Math|Vector|MakeVector 0.0 0.0 (Variables|Default|GetTemp_Height)) "0, 0, 0" "0.060000,0.500000,0.070000") false)
    (Variables|Default|SetTemp_Height (+ (Variables|Default|GetTemp_Height) (Variables|Default|GetStep%20Gap)))
    (AddComponent|AddBoxComponent false (Math|Transform|MakeTransform (Math|Vector|MakeVector 0.0 0.0 (/ (Variables|Default|GetHeight) 2.0)) "0, 0, 0" (Math|Vector|MakeVector 0.4 1.2 (/ (Variables|Default|GetHeight) 64.0))))
    (AddComponent|AddArrowComponent false (Variables|Default|GetLadderTop))
    (AddComponent|AddArrowComponent false (Variables|Default|GetLadderBottom))))